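; Base enemy for the space shooter that flies along its initial forward direction and fires on a timer.
; Tick moves it without sweep and spawns Ammo at FirePoint, aligned to the enemy's rotation.
; Overlapping the player character damages it and plays a collapse sound.
; The OnEnemyDestroy dispatcher triggers delayed self-destruction; the tag check that would call it and notify SS_GameMode is unconnected.
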(event `self.ReceiveBeginPlay`
  ; Setup Initial Direction and Destroy Event
  (set `self.MovementVector` (`self.GetActorForwardVector`))
  (add `self.OnEnemyDestroy` (delegate `Destroyed_Event`)))

(event `Destroyed_Event`
  ; Setup Initial Direction and Destroy Event
  (`KismetSystemLibrary.Delay` 0.2)
  (`self.K2_DestroyActor`))

(event `self.ReceiveTick`
  (params (DeltaSeconds :type "Float (single-precision)"))
  ; Update Movement and Fire
  (`self.Move` DeltaSeconds)
  (bind _output_get (set `self.ShotCurrentTime` (+ DeltaSeconds (`self.ShotCurrentTime`))))
  (if (> _output_get (`self.DelayShoot`))
    (set `self.ShotCurrentTime` 0.0)
    (`self.Fire`)))

(event `self.ReceiveActorBeginOverlap`
  (params (OtherActor :type "Actor Object Reference"))
  (bind _asbp_space_s_character (cast `/Game/SpaceShooter/Player/BP_SpaceS_Character` OtherActor))
  (`/Game/SpaceShooter/Player/BP_SpaceS_Character.TakeDamage` _asbp_space_s_character)
  (`GameplayStatics.PlaySound2D` "/Game/StarterContent/Audio/Collapse_Cue.Collapse_Cue" 1.0 1.0 0.0 null null))

(fn `Fire`
  (bind _returnvalue (`|SpawnActorFromClass` (`self.Ammo`) (`SceneComponent.K2_GetComponentToWorld` (`self.FirePoint`)) "Undefined" "MultiplyWithRoot" null null))
  (`GameplayStatics.PlaySoundAtLocation` "/Game/SpaceShooter/Audio/shot_2.shot_2" (0.0 0.0 0.0) (struct) 0.2 1.0 0.0 null null null null)
  (`self.K2_SetActorRotation` _returnvalue (`self.K2_GetActorRotation`) false))

(fn `Move`
  (params (DeltaTime :type "Float (double-precision)"))
  (`self.K2_SetActorLocation` (+ (`self.K2_GetActorLocation`) (* (* DeltaTime (`self.Speed`)) (`self.MovementVector`)))))

(fn `UserConstructionScript`)