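; Enemy spawner actor for the space shooter that spawns enemies on a looping timer at random components tagged SpawnPoint.
; It randomly picks base or horizontal enemies, adds sine enemies once GameMode Progress is high enough, and substitutes base when horizontal ones hit a cap.
; The level-based Type input goes unused.
; Each enemy's destroy event lowers SpawnTime, but the running timer is never reset with the new value.
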(event `self.ReceiveBeginPlay`
  (`KismetSystemLibrary.K2_SetTimerDelegate` (delegate `Spawn`) (`self.SpawnTime`) true)
  (bind _asss_game_mode (cast `/Game/SpaceShooter/SS_GameMode` (`GameplayStatics.GetGameMode`)))
  (set `self.SS_Game Mode` _asss_game_mode))

(event `Spawn`
  (bind _enemyspawned (`self.SpawnEnemy`))
  (`/Engine/EditorBlueprintResources/StandardMacros.IsValid` _enemyspawned
    (:`Is Valid`
      (add `/Game/SpaceShooter/Enemies/BP_EnemyBase.OnEnemyDestroy` _enemyspawned (delegate `EnemyDestroyed`)))))

(event `EnemyDestroyed`
  (set `self.SpawnTime` (- (`self.SpawnTime`) 1.0)))

(fn `GetClasstoSpawn`
  (params (Type :type Integer))
  (returns (Clase :type "Actor Class Reference"))
  (return (select `int` (`KismetMathLibrary.RandomInteger` (`KismetMathLibrary.SelectInt` 3 2 (>= (`/Game/SpaceShooter/SS_GameMode.Progress` (cast `/Game/SpaceShooter/SS_GameMode` (`GameplayStatics.GetGameMode`) :!pure true)) 10))) :`0` "/Game/SpaceShooter/Enemies/BP_EnemyBase.BP_EnemyBase_C" :`1` "/Game/SpaceShooter/Enemies/BP_Enemy_Horizontal.BP_Enemy_Horizontal_C" :`2` "/Game/SpaceShooter/Enemies/BP_Enemy_Sine.BP_Enemy_Sine_C" :!type "Actor Class Reference")))

(fn `SpawnEnemy`
  (returns (EnemySpawned :type "/Game/SpaceShooter/Enemies/BP_EnemyBase Object Reference"))
  (bind _returnvalue (`self.GetComponentsByTag` "/Script/Engine.SceneComponent" "SpawnPoint"))
  (bind _clase (`self.GetClasstoSpawn` (`KismetMathLibrary.RandomInteger` (+ (`/Game/SpaceShooter/SS_GameMode.Level` (`self.SS_Game Mode`)) 0))))
  (bind _outactors (`GameplayStatics.GetAllActorsOfClass` "/Game/SpaceShooter/Enemies/BP_Enemy_Horizontal.BP_Enemy_Horizontal_C"))
  (bind _returnvalue_2 (`|SpawnActorFromClass` (select `bool` (and (== _clase "/Game/SpaceShooter/Enemies/BP_Enemy_Horizontal.BP_Enemy_Horizontal_C") (>= (`KismetArrayLibrary.Array_Length` _outactors) 10)) :`false` _clase :`true` "/Game/SpaceShooter/Enemies/BP_EnemyBase.BP_EnemyBase_C") (`SceneComponent.K2_GetComponentToWorld` (`|GetArrayItem` _returnvalue (`KismetMathLibrary.RandomInteger` (`KismetArrayLibrary.Array_Length` _returnvalue)))) "AdjustIfPossibleButAlwaysSpawn" "MultiplyWithRoot" null null))
  (bind _asbp_enemy_base (cast `/Game/SpaceShooter/Enemies/BP_EnemyBase` _returnvalue_2))
  (return _asbp_enemy_base))

(fn `UserConstructionScript`)