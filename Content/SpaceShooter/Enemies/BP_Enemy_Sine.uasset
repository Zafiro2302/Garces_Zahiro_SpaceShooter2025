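; BP_Enemy_Sine is a space shooter enemy that weaves side to side along world Y in a sine wave.
; It stores its starting Y at BeginPlay as the center of the wave.
; Each Tick runs the parent logic, accumulates running time, then sets Y from the sine speed and amplitude while keeping the current X and Z.
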(event `self.ReceiveBeginPlay`
  (bind (_returnvalue_x _returnvalue_y) (`KismetMathLibrary.BreakVector` (`self.K2_GetActorLocation`)))
  (`parent.ReceiveBeginPlay`)
  (set `self.InitialY` _returnvalue_y))

(event `self.ReceiveTick`
  (params (DeltaSeconds :type "Float (single-precision)"))
  (bind (_returnvalue_x _returnvalue_y _returnvalue_z) (`KismetMathLibrary.BreakVector` (`self.K2_GetActorLocation`)))
  (`parent.ReceiveTick` DeltaSeconds)
  (bind _output_get (set `self.RunningTime` (+ (`self.RunningTime`) DeltaSeconds)))
  (`self.K2_SetActorLocation` (`KismetMathLibrary.MakeVector` _returnvalue_x (+ (* (`KismetMathLibrary.Sin` (* _output_get (`self.SineSpeed`))) (`self.SineAmplitude`)) (`self.InitialY`)) _returnvalue_z)))

(fn `UserConstructionScript`
  (`parent.UserConstructionScript`))