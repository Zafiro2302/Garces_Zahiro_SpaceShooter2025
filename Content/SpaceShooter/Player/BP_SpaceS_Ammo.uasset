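; BP_SpaceS_Ammo is a space shooter projectile that flies forward at its Speed, moved every Tick without sweep.
; On overlap it ignores Pawns; any other actor that casts to BP_EnemyBase is destroyed after SS_GameMode's EnemyDestroy is notified.
; The hit spawns an explosion emitter and sound at the projectile, which destroys itself after a short delay.
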(event `self.ReceiveActorBeginOverlap`
  (params (OtherActor :type "Actor Object Reference"))
  ; OnCollision
  (cast `Pawn` OtherActor
    (:`CastFailed`
      (bind _asbp_enemy_base (cast `/Game/SpaceShooter/Enemies/BP_EnemyBase` OtherActor))
      (bind _asss_game_mode (cast `/Game/SpaceShooter/SS_GameMode` (`GameplayStatics.GetGameMode`)))
      (`/Game/SpaceShooter/SS_GameMode.EnemyDestroy` _asss_game_mode)
      (`self.K2_DestroyActor` _asbp_enemy_base)
      (`GameplayStatics.SpawnEmitterAtLocation` "/Game/StarterContent/Particles/P_Explosion.P_Explosion" (`self.K2_GetActorLocation`))
      (`GameplayStatics.PlaySound2D` "/Game/StarterContent/Audio/Explosion01.Explosion01" 0.5 1.0 0.0 null null)
      (`KismetSystemLibrary.Delay` 0.2)
      (`self.K2_DestroyActor`))))

(event `self.ReceiveTick`
  (params (DeltaSeconds :type "Float (single-precision)"))
  ; Update Movement
  (`self.K2_SetActorLocation` (+ (`self.K2_GetActorLocation`) (* (`self.GetActorForwardVector`) (* DeltaSeconds (`self.Speed`))))))

(fn `UserConstructionScript`)