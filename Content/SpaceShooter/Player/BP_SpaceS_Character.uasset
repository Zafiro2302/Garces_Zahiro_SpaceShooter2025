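; Player ship character for the SpaceShooter game, handling movement, shooting and lives.
; Enhanced Input drives planar movement and timer-throttled fire, which spawns BP_SpaceS_Ammo at FireSpawn.
; An enabled triple-shot upgrade instead spawns three short-lived projectiles, the outer two angled in yaw.
; Taking damage removes a life and grants brief invulnerability, or reports player death to SS_GameMode when none remain.
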(event `self.ReceiveBeginPlay`
  (bind _asplayer_controller (cast `PlayerController` (`self.GetController`)))
  (bind _returnvalue (pcsubsystem `EnhancedInputLocalPlayerSubsystem` _asplayer_controller))
  (`/Engine/EditorBlueprintResources/StandardMacros.IsValid` _returnvalue
    (:`Is Valid`
      (`EnhancedInputSubsystemInterface.AddMappingContext` _returnvalue "/Game/SpaceShooter/Input/IMC_Player.IMC_Player" 0 (struct)))))

(event `self.ReceiveActorBeginOverlap`
  (params (OtherActor :type "Actor Object Reference")))

(event `EnhancedInput|/Game/SpaceShooter/Input/IA_Player_Fire`
  (params (ActionValue :type Boolean) (ElapsedSeconds :type "Float (double-precision)") (TriggeredSeconds :type "Float (double-precision)") (InputAction :type "InputAction Object Reference" :default "/Game/SpaceShooter/Input/IA_Player_Fire.IA_Player_Fire"))
  (:`Triggered`
    (if (`self.CanFire`)
      (`self.DoFire`)
      (set `self.CanFire` false)
      (`KismetSystemLibrary.K2_SetTimerDelegate` (delegate `EnableFire`) (`self.FireDelay`)))))

(event `EnableFire`
  (set `self.CanFire` true))

(event `EnhancedInput|/Game/SpaceShooter/Input/IA_Player_Movement`
  (params (ActionValue :type "Vector2D Structure") (ElapsedSeconds :type "Float (double-precision)") (TriggeredSeconds :type "Float (double-precision)") (InputAction :type "InputAction Object Reference" :default "/Game/SpaceShooter/Input/IA_Player_Movement.IA_Player_Movement"))
  (:`Triggered`
    (`self.AddMovementInput` (`self.GetActorRightVector`) ActionValue_X)
    (`self.AddMovementInput` (`self.GetActorForwardVector`) ActionValue_Y)))

(event `DamageActor`
  (bind _asss_game_mode (cast `/Game/SpaceShooter/SS_GameMode` (`GameplayStatics.GetGameMode`)))
  (`/Game/SpaceShooter/SS_GameMode.PlayerDead` _asss_game_mode))

(event `TakeDamage`
  (if (not (`self.IsInvulnerable`))
    (set `self.IsInvulnerable` true)
    (set `self.Lifes` (- (`self.Lifes`) 1))
    (if (<= (`self.Lifes`) 0)
      (`self.DamageActor`)
      (else
        (`|ExecutionSequence`
          (:`then_1`
            (`KismetSystemLibrary.Delay` 1.0)
            (set `self.IsInvulnerable` false)))))))

(event `EnableTripleShot`
  (set `self.HasTripleShot` true))

(fn `DoFire`
  (bind _firespawn (`self.FireSpawn`))
  (bind _returnvalue (`SceneComponent.K2_GetComponentLocation` _firespawn))
  (bind _roll (.roll (`SceneComponent.K2_GetComponentRotation` _firespawn)))
  (bind _pitch (.pitch (`SceneComponent.K2_GetComponentRotation` _firespawn)))
  (bind _yaw (.yaw (`SceneComponent.K2_GetComponentRotation` _firespawn)))
  (`GameplayStatics.PlaySound2D` "/Game/SpaceShooter/Audio/shot_1.shot_1" 0.2 1.0 0.0 null null)
  (if (`self.HasTripleShot`)
    (bind _returnvalue_2 (`|SpawnActorFromClass` "/Game/SpaceShooter/Player/BP_SpaceS_Ammo.BP_SpaceS_Ammo_C" (`KismetMathLibrary.Conv_VectorToTransform` _returnvalue) "Undefined" "MultiplyWithRoot" null null))
    (`self.SetLifeSpan` _returnvalue_2 0.5)
    (bind _returnvalue_3 (`|SpawnActorFromClass` "/Game/SpaceShooter/Player/BP_SpaceS_Ammo.BP_SpaceS_Ammo_C" (`KismetMathLibrary.MakeTransform` _returnvalue (`KismetMathLibrary.MakeRotator` _roll _pitch (- _yaw 20.0))) "Undefined" "MultiplyWithRoot" null null))
    (`self.SetLifeSpan` _returnvalue_3 0.5)
    (bind _returnvalue_4 (`|SpawnActorFromClass` "/Game/SpaceShooter/Player/BP_SpaceS_Ammo.BP_SpaceS_Ammo_C" (`KismetMathLibrary.MakeTransform` _returnvalue (`KismetMathLibrary.MakeRotator` _roll _pitch (+ _yaw 20.0))) "Undefined" "MultiplyWithRoot" null null))
    (`self.SetLifeSpan` _returnvalue_4 0.5)
    (else
      (`|SpawnActorFromClass` "/Game/SpaceShooter/Player/BP_SpaceS_Ammo.BP_SpaceS_Ammo_C" (`SceneComponent.K2_GetComponentToWorld` (`self.FireSpawn`)) "Undefined" "MultiplyWithRoot" null null))))

(fn `UserConstructionScript`)